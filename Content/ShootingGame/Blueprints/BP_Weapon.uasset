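; BP_Weapon is a gun actor for the shooting game, with a static mesh whose collision is disabled on BeginPlay.
; PullTrigger plays a single-shot rifle montage on the owning character.
; DoShoot spawns a small explosion particle at the mesh's muzzle socket and an explosion sound at the actor's location, with no projectile or damage logic.
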(event EventBeginPlay
  (Collision|SetCollisionEnabled (Variables|Default|GetStaticMesh) "NoCollision"))

(fn ConstructionScript)

(fn DoShoot
  (bind _staticmesh (Variables|Default|GetStaticMesh))
  (Effects|SpawnEmitteratLocation "/Game/StarterContent/Particles/P_Explosion.P_Explosion" (Transformation|GetSocketLocation _staticmesh "muzzle") (Transformation|GetSocketRotation _staticmesh "muzzle") "0.100000,0.100000,0.100000")
  (Audio|SpawnSoundatLocation "/Game/StarterContent/Audio/Explosion01.Explosion01" (Transformation|GetActorLocation) "0, 0, 0" 1.0 1.0 0.0 0 0))

(fn PullTrigger
  (Animation|PlayAnimMontage (Variables|Default|GetOwnCharacter) "/Game/Characters/Mannequins/Animations/RifleAnimPro/InPlace/Rifle_ShootOnce_Montage.Rifle_ShootOnce_Montage" 1.0 "None"))